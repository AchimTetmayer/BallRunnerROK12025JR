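; BP_TP is a tilting platform that pitches its Cube while the player's BP_Ball is inside its Box trigger.
; Box begin overlap sets IsTilting only for the player's ball, while any end overlap clears it.
; Each Tick uses FInterpTo at TiltSpeed to ease the Cube's relative pitch toward Tiltangle, or back to level when not tilting, holding roll and yaw at zero.
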(event `self.Box.OnComponentBeginOverlap`
  (params (OverlappedComponent :type "PrimitiveComponent Object Reference") (OtherActor :type "Actor Object Reference") (OtherComp :type "PrimitiveComponent Object Reference") (OtherBodyIndex :type Integer) (bFromSweep :type Boolean) (SweepResult :type "HitResult Structure (by ref)"))
  ;[0.5158 1 0] Overlap Detect
  (bind _asbp_ball (cast `/Game/BP_Ball` (`GameplayStatics.GetPlayerPawn` 0)))
  (if (== _asbp_ball OtherActor)
    (set `self.IsTilting` true)))

(event `self.Box.OnComponentEndOverlap`
  (params (OverlappedComponent :type "PrimitiveComponent Object Reference") (OtherActor :type "Actor Object Reference") (OtherComp :type "PrimitiveComponent Object Reference") (OtherBodyIndex :type Integer))
  ;[0.5158 1 0] Overlap Detect
  (set `self.IsTilting` false))

(event `self.ReceiveTick`
  (params (DeltaSeconds :type "Float (single-precision)"))
  (bind _returnvalue (* DeltaSeconds 0.1))
  (bind _tiltspeed (`self.TiltSpeed`))
  (bind _cube (`self.Cube`))
  (bind (_relativerotation_roll _relativerotation_pitch) (`KismetMathLibrary.BreakRotator` (`SceneComponent.RelativeRotation` _cube)))
  ;[0.948 1 0] Movement Y
  (if (`self.IsTilting`)
    (`SceneComponent.K2_SetRelativeRotation` _cube (`KismetMathLibrary.MakeRotator` 0.0 (`KismetMathLibrary.FInterpTo` _relativerotation_pitch (`self.Tiltangle`) _returnvalue _tiltspeed)) false false)
    (else
      (`SceneComponent.K2_SetRelativeRotation` _cube (`KismetMathLibrary.MakeRotator` 0.0 (`KismetMathLibrary.FInterpTo` _relativerotation_pitch 0.0 _returnvalue _tiltspeed)) false false))))

(fn `UserConstructionScript`)