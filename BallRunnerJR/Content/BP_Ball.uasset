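; BP_Ball is a physics-driven ball moved by player input, with a zoomable spring arm.
; The WS and AD axes share one torque call on the Sphere, applying the same axis value to both X and Y as acceleration.
; The left-mouse action applies an upward impulse of Jumpheight and clears CanJump, which this graph never checks or resets.
; The mouse wheel shortens or lengthens the spring arm in fixed, unclamped steps.
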(event `Key|MouseScrollUp`
  (params (Key :type "Key Structure"))
  (bind _springarm (`self.SpringArm`))
  (:`Pressed`
    (set `SpringArmComponent.TargetArmLength` (+ (`SpringArmComponent.TargetArmLength` _springarm) -5.0) _springarm)))

(event `Key|MouseScrollDown`
  (params (Key :type "Key Structure"))
  (bind _springarm (`self.SpringArm`))
  (:`Pressed`
    (set `SpringArmComponent.TargetArmLength` (+ (`SpringArmComponent.TargetArmLength` _springarm) 5.0) _springarm)))

(event `InputAxis|AxisMap_WS`
  (params (AxisValue :type "Float (single-precision)"))
  (`PrimitiveComponent.AddTorqueInRadians` (`self.Sphere`) (`KismetMathLibrary.MakeVector` (* AxisValue 10.0) (* (stale `InputAxis|AxisMap_AD` AxisValue) 10.0)) "None" true :!label _label))

(event `InputAxis|AxisMap_AD`
  (params (AxisValue :type "Float (single-precision)"))
  (goto _label))

(event `InputAction|ActionMAP_LMB`
  (params (Key :type "Key Structure"))
  (:`Pressed`
    (`PrimitiveComponent.AddImpulse` (`self.Sphere`) (`KismetMathLibrary.MakeVector` 0.0 0.0 (`self.Jumpheight`)) "None" false)
    (set `self.CanJump` false)))

(fn `UserConstructionScript`)