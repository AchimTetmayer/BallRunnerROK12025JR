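; BP_Ball is a player-controlled physics ball that rolls, jumps and carries an orbiting, zoomable spring-arm camera.
; Tick rotates the spring arm from axis input with roll locked, while the mouse wheel changes arm length.
; WASD axes apply torque relative to camera yaw, so steering follows the view.
; Space or left mouse adds an upward impulse through a shared DoOnce, reset by a delay after release rather than a ground check.
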(event `self.ReceiveTick`
  (params (DeltaSeconds :type "Float (single-precision)"))
  (bind _springarm (`self.SpringArm`))
  (bind (_returnvalue_roll _returnvalue_pitch _returnvalue_yaw) (`KismetMathLibrary.BreakRotator` (`SceneComponent.K2_GetComponentRotation` _springarm)))
  ;[1 1 1] Camera Movement
  (`SceneComponent.K2_SetWorldRotation` _springarm (`KismetMathLibrary.MakeRotator` 0.0 (+ _returnvalue_pitch (`self.GetInputAxisKeyValue`)) (+ _returnvalue_yaw (`self.GetInputAxisKeyValue`))) false false))

(event `Key|MouseScrollUp`
  (params (Key :type "Key Structure"))
  (bind _springarm (`self.SpringArm`))
  ;[1 0.2855 0] Camera In/Out
  (:`Pressed`
    (set `SpringArmComponent.TargetArmLength` (+ (`SpringArmComponent.TargetArmLength` _springarm) (* (`self.CameraZoomSpeed`) -1.0)) _springarm)))

(event `Key|MouseScrollDown`
  (params (Key :type "Key Structure"))
  (bind _springarm (`self.SpringArm`))
  ;[1 0.2855 0] Camera In/Out
  (:`Pressed`
    (set `SpringArmComponent.TargetArmLength` (+ (`SpringArmComponent.TargetArmLength` _springarm) (`self.CameraZoomSpeed`)) _springarm)))

(event `InputAxis|AxisMap_AD`
  (params (AxisValue :type "Float (single-precision)"))
  (bind (_returnvalue_roll _returnvalue_pitch _returnvalue_yaw) (`KismetMathLibrary.BreakRotator` (`SceneComponent.K2_GetComponentRotation` (`self.Camera`))))
  ;[1 1 1] Steering Left/Right
  (`PrimitiveComponent.AddTorqueInRadians` (`self.Sphere`) (* (`KismetMathLibrary.GetRightVector` (`KismetMathLibrary.MakeRotator` 0.0 0.0 (+ _returnvalue_yaw 90.0))) (* AxisValue (`self.BallSpeed`))) "None" true))

(event `InputAxis|AxisMap_WS`
  (params (AxisValue :type "Float (single-precision)"))
  (bind (_returnvalue_roll _returnvalue_pitch _returnvalue_yaw) (`KismetMathLibrary.BreakRotator` (`SceneComponent.K2_GetComponentRotation` (`self.Camera`))))
  (bind (_returnvalue_x _returnvalue_y) (`KismetMathLibrary.BreakVector` (* (`KismetMathLibrary.GetRightVector` (`KismetMathLibrary.MakeRotator` 0.0 0.0 _returnvalue_yaw)) (* AxisValue (`self.BallSpeed`)))))
  ;[1 1 1] Steering Forward/Back
  (`PrimitiveComponent.AddTorqueInRadians` (`self.Sphere`) (`KismetMathLibrary.MakeVector` _returnvalue_x _returnvalue_y) "None" true))

(event `Key|SpaceBar`
  (params (Key :type "Key Structure"))
  ;[1 0.898 0] Jump Z
  (:`Pressed`
    (`/Engine/EditorBlueprintResources/StandardMacros.DoOnce` false :!label _label
      (:`Completed`
        (`PrimitiveComponent.AddImpulse` (`self.Sphere`) (`KismetMathLibrary.MakeVector` 0.0 0.0 (`self.JumpHeight`)) "None" true))))
  (:`Released`
    (`KismetSystemLibrary.Delay` 1.2 :!label _label_2)
    (goto _label :!via `Reset`)))

(event `InputAction|ActionMAP_LMB`
  (params (Key :type "Key Structure"))
  ;[1 0.898 0] Jump Z
  (:`Pressed`
    (goto _label))
  (:`Released`
    (goto _label_2)))

(fn `UserConstructionScript`)